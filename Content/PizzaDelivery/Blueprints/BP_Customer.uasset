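; BP_Customer is a pizza delivery target that resolves a delivery when the player's moped overlaps it.
; On BeginPlay it sizes its sphere to DetectionRadius.
; When a BP_MopedCharacter overlaps and holds at least CurrentRequest pizzas, it takes them, reports success for its AssignedLocation to the CustomerSpawner and destroys itself.
; Scoring is only a debug-print placeholder, and too few pizzas just prints a message.
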(event EventBeginPlay
  (Components|Sphere|SetSphereRadius (Variables|Default|GetSphere) (Variables|Default|GetDetectionRadius) true))

(event Collision|EventActorBeginOverlap
  (params (OtherActor :type Actor%20Object%20Reference))
  (bind _customer_spawner (Variables|Default|GetCustomer%20Spawner))
  (bind _asbp_moped_character (Utilities|Casting|CastToBP_MopedCharacter OtherActor))
  (Utilities|IsValid _customer_spawner
    (:Is%20Valid
      (if (>= (Default|HowManyPizzas? _asbp_moped_character) (Variables|Default|GetCurrent%20%20Request))
        (Development|PrintString "Handle Scoring Here")
        (Default|DeliverPizza _asbp_moped_character (Variables|Default|GetCurrent%20%20Request))
        (Default|DeliverySuccessful _customer_spawner (Variables|Default|GetAssigned%20Location))
        (Actor|DestroyActor)
        (else
          (Development|PrintString "Not Enough Pizzas!"))))))

(event EventTick
  (params (DeltaSeconds :type Float%20%28single-precision%29)))

(fn ConstructionScript)