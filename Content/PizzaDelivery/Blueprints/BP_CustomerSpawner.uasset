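; Customer spawner for the pizza delivery game that creates a customer at BeginPlay and another after each successful delivery.
; It picks a random TargetPoint tagged "Empty", spawns BP_Customer there with spawner and location references, and removes the tag to reserve it.
; Each spawn sets and prints a one-pizza request and clears the restaurant's fulfilled-order flag.
; DeliverySuccessful re-tags the delivered location as empty after generating the next customer.
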(event Custom|Delivery%20Successful
  (params (Location%20Delivered%20To :type Target%20Point%20Object%20Reference))
  (CallFunction|GenerateNewCustomer)
  (Utilities|IsValid Location%20Delivered%20To
    (:Is%20Valid
      (Utilities|Array|Add (Variables|/Script/Engine.Actor|GetTags Location%20Delivered%20To) "Empty"))))

(event EventBeginPlay
  (CallFunction|GenerateNewCustomer))

(event EventTick
  (params (DeltaSeconds :type Float%20%28single-precision%29)))

(fn ConstructionScript)

(fn GenerateNewCustomer
  ;[1 1 1] Find all Target Points with the "Empty" Tag
  (bind _outactors (Actor|GetAllActorsOfClasswithTag "/Script/Engine.TargetPoint" "Empty"))
  (bind _output_get (LocalVariables|SetAvailable%20Locations _outactors))
  (if (> (Utilities|Array|Length _output_get) 0)
    ;[1 1 1] Spawn a Customer at the randomly selected TargetPoint (Available Location)
    (bind _output_get_2 (LocalVariables|SetSelected%20Location (.OutItem (Utilities|Array|Random (LocalVariables|GetAvailable%20Locations)))))
    (bind _returnvalue (Game|SpawnActorfromClass "/Game/PizzaDelivery/Blueprints/BP_Customer.BP_Customer_C" (Transformation|GetActorTransform _output_get_2) "Undefined" "MultiplyWithRoot" 0 0))
    ;[1 1 1] Update new Customer with the Spawner Obj and Assigned Location, and then remove the "Empty" Tag so the location cannot be reused while occupied by a customer.
    (Variables|/Game/PizzaDelivery/Blueprints/BP_Customer.BP_Customer_C|SetCustomer%20Spawner _returnvalue self)
    (bind _output_get_3 (Variables|/Game/PizzaDelivery/Blueprints/BP_Customer.BP_Customer_C|SetAssigned%20Location _returnvalue (LocalVariables|GetSelected%20Location)))
    (Utilities|Array|RemoveItem (Variables|/Script/Engine.Actor|GetTags _output_get_3) "Empty")
    (bind _output_get_4 (Variables|/Game/PizzaDelivery/Blueprints/BP_Customer.BP_Customer_C|SetCurrent%20%20Request _returnvalue 1))
    (bind _output_get_5 (Variables|Default|SetCurrent%20Customer%20Request _output_get_4))
    ;[1 1 1] Set the Current Customer Request
    (Development|PrintString (Utilities|String|Append "Customer Requests " (Utilities|String|ToString(Integer) _output_get_5) " Pizza(s)."))
    ;[1 1 1] Clearing Order FullFilled Flag in Pizza Restaurant so Player can collect a new Order (Flag should also be cleared when the player takes damage)
    (bind _returnvalue_2 (Actor|GetActorOfClass "/Game/PizzaDelivery/Blueprints/BP_PizzaRestaurant.BP_PizzaRestaurant_C"))
    (Variables|/Game/PizzaDelivery/Blueprints/BP_PizzaRestaurant.BP_PizzaRestaurant_C|SetOrder%20Fullfilled? _returnvalue_2 false)
    (return true)
    (else
      (return false))))