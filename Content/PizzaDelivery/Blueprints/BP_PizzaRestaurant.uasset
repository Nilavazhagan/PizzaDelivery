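; BP_PizzaRestaurant is a healing spot that restores any DamageableActor overlapping it to full health.
; HealCharacter plays a restore sound and, for a moped character, resets max speed to normal.
; The overlap then updates the HUD health display and stops the player moped's last-stand sound.
; BeginPlay caches the level's customer spawner, though nothing here uses it.
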(event EventBeginPlay
  (bind _returnvalue (Actor|GetActorOfClass "/Game/PizzaDelivery/Blueprints/BP_CustomerSpawner.BP_CustomerSpawner_C"))
  (Variables|Default|SetCustomer%20Spawner _returnvalue))

(event Collision|EventActorBeginOverlap
  (params (OtherActor :type Actor%20Object%20Reference))
  (bind _asdamageable_actor (Utilities|Casting|CastToDamageableActor OtherActor))
  (CallFunction|HealCharacter _asdamageable_actor)
  ;[1 1 1] Update UI
  (bind _asbp_hud (Utilities|Casting|CastToBP_HUD (HUD|GetHUD (Game|GetPlayerController 0))))
  (bind _returnvalue (Class|DamageableActor|GetHealth _asdamageable_actor))
  (Default|OnPlayerHealthChanged (Variables|/Game/PizzaDelivery/UI/BP_HUD.BP_HUD_C|GetHUDReference _asbp_hud) _returnvalue)
  (bind _asbp_moped_character (Utilities|Casting|CastToBP_MopedCharacter (Game|Player|GetPlayerPawn 0)))
  (Audio|Components|Audio|Stop (Variables|/Game/TopDown/Blueprints/BP_MopedCharacter.BP_MopedCharacter_C|GetLastStandSound _asbp_moped_character)))

(event EventTick
  (params (DeltaSeconds :type Float%20%28single-precision%29)))

(fn ConstructionScript)

(fn HealCharacter
  (params (Player%20Char :type Damageable%20Actor%20Object%20Reference))
  (Utilities|IsValid Player%20Char
    (:Is%20Valid
      (Class|DamageableActor|FullyHealCharacter Player%20Char)
      (Audio|PlaySoundatLocation "/Game/PizzaDelivery/SFX/Gameplay/Hp_Restored.Hp_Restored" (Transformation|GetActorLocation) "0, 0, 0" 1.0 1.0 0.0 0 0 0 0)
      (bind _asbp_moped_character (Utilities|Casting|CastToBP_MopedCharacter Player%20Char))
      (Variables|/Game/TopDown/Blueprints/BP_MopedCharacter.BP_MopedCharacter_C|SetMaxSpeed _asbp_moped_character (Variables|/Game/TopDown/Blueprints/BP_MopedCharacter.BP_MopedCharacter_C|GetNormalMaxSpeed _asbp_moped_character))
      (return true))
    (:Is%20Not%20Valid
      (return false))))